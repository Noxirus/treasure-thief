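; BP_SplinePlatform is a moving platform that travels continuously between the points of its PlatformPath spline.
; A timeline drives a straight-line lerp of the mesh's relative location between consecutive points, ignoring spline curvature, with the same duration per segment.
; Each time the timeline finishes, it advances the point index and replays.
; At the last point, the index either wraps to zero when Looping or reverses to ping-pong along the path.
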(event EventBeginPlay
  (Variables|Default|SetOrigin (Variables|/Script/Engine.SceneComponent|GetRelativeLocation (Variables|Default|GetPlatformMesh)))
  (CallFunction|SetLocations)
  (bind _movetrack (Timeline|MovingTimeline Play)
    (:Update
      (CallFunction|MovePlatform _movetrack))
    (:Finished
      (CallFunction|SetLocations)
      (Components|Timeline|PlayfromStart (Variables|Default|GetMovingTimeline)))))

(fn ConstructionScript)

(fn MovePlatform
  (params (Alpha :type Float%20%28single-precision%29))
  (Transformation|SetRelativeLocation (Variables|Default|GetPlatformMesh) (Math|Vector|Lerp(Vector) (Variables|Default|GetOrigin) (Variables|Default|GetSplineDestination) Alpha) false false))

(fn SetLocations
  (Variables|Default|SetOrigin (Spline|GetLocationatSplinePoint (Variables|Default|GetPlatformPath) (Variables|Default|GetCurrentPathIndex) "Local"))
  (CallFunction|IterateSplineIndex)
  (Variables|Default|SetSplineDestination (Spline|GetLocationatSplinePoint (Variables|Default|GetPlatformPath) (Variables|Default|GetCurrentPathIndex) "Local")))

(fn IterateSplineIndex
  (if (Variables|Default|GetbMovingForward)
    (if (CallFunction|AtEndOfPath)
      (if (Variables|Default|GetbLooping)
        (Variables|Default|SetCurrentPathIndex 0)
        (else
          (Variables|Default|SetbMovingForward false)
          (Math|Integer|DecrementInt (Variables|Default|GetCurrentPathIndex))))
      (else
        (Math|Integer|IncrementInt (Variables|Default|GetCurrentPathIndex))))
    (elif (<= (Variables|Default|GetCurrentPathIndex) 0)
      (Variables|Default|SetbMovingForward true)
      (Math|Integer|IncrementInt (Variables|Default|GetCurrentPathIndex))
      (else
        (Math|Integer|DecrementInt (Variables|Default|GetCurrentPathIndex))))))

(fn AtEndOfPath
  (return (>= (Variables|Default|GetCurrentPathIndex) (- (Spline|GetNumberOfSplinePoints (Variables|Default|GetPlatformPath)) 1))))