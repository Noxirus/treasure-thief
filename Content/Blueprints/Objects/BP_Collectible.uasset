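; BP_Collectible is a treasure pickup that registers its collection with the treasure game mode.
; Its construction script sets the mesh by looking up TreasureType in the TreasureMeshs map.
; When a DefaultPawn overlaps the trigger, it calls CollectTreasure on BP_TreasureGameMode and destroys itself.
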(event OnComponentBeginOverlap(OverlapTrigger)
  (params (OverlappedComponent :type Primitive%20Component%20Object%20Reference) (OtherActor :type Actor%20Object%20Reference) (OtherComp :type Primitive%20Component%20Object%20Reference) (OtherBodyIndex :type Integer) (bFromSweep :type Boolean) (SweepResult :type Hit%20Result%20Structure%20%28by%20ref%29))
  (Utilities|Casting|CastToDefaultPawn OtherActor)
  (bind _asbp_treasure_game_mode (Utilities|Casting|CastToBP_TreasureGameMode (Game|GetGameMode)))
  (Default|CollectTreasure _asbp_treasure_game_mode)
  (Actor|DestroyActor))

(fn ConstructionScript
  (CallFunction|UpdateTreasureMesh (Variables|Default|GetTreasureType)))

(fn UpdateTreasureMesh
  (params (TreasureType :type E_TreasureType%20Enum :default "NewEnumerator0"))
  (Components|StaticMesh|SetStaticMesh (Variables|Default|GetCollectibleMesh) (.Value (Utilities|Map|Find (Variables|Default|GetTreasureMeshs) TreasureType))))