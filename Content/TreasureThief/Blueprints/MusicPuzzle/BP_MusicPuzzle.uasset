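; BP_MusicPuzzle is a music puzzle Blueprint that checks entered notes against an answer sequence.
; AddNewNote appends each note to CurrentAnswer and compares the sequence element by element with MusicAnswer.
; A mismatch clears CurrentAnswer, and reaching the full answer length counts as solved.
; Both outcomes only print debug strings; no other gameplay response is wired.
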(fn ConstructionScript)

(fn AddNewNote
  (params (NoteToAdd :type Integer))
  (Utilities|Array|Add (Variables|Default|GetCurrentAnswer) NoteToAdd)
  (for (_array_element _array_index) (Variables|Default|GetCurrentAnswer)
    (if (!= _array_element (Utilities|Array|Get(acopy) (Variables|Default|GetMusicAnswer) _array_index))
      (Utilities|Array|Clear (Variables|Default|GetCurrentAnswer))
      (Development|PrintString "WRONG1")))
  (if (== (Utilities|Array|Length (Variables|Default|GetMusicAnswer)) (Utilities|Array|Length (Variables|Default|GetCurrentAnswer)))
    (Development|PrintString "Was Correct!")))