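; BP_Guard is a guard Blueprint that currently visualizes its orientation relative to the player goblin using vector math debug output.
; It caches the BP_PlayerGoblin on BeginPlay, then every tick prints the dot product of its forward vector and the direction to the player.
; It also draws a debug line along the cross product of the player's and guard's forward vectors.
; No detection response or movement is implemented.
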(event EventTick
  (params (DeltaSeconds :type Float%20%28single-precision%29))
  (CallFunction|DotProduct)
  (CallFunction|CrossProduct))

(event EventBeginPlay
  (bind _returnvalue (Actor|GetActorOfClass "/Game/TreasureThief/Blueprints/Characters/BP_PlayerGoblin.BP_PlayerGoblin_C"))
  (Variables|Default|SetPlayer _returnvalue))

(fn ConstructionScript)

(fn DotProduct
  (Development|PrintString (Utilities|String|ToString(Float) (Math|Vector|DotProduct (Math|Vector|Normalize (- (Transformation|GetActorLocation (Variables|Default|GetPlayer)) (Transformation|GetActorLocation))) (Transformation|GetActorForwardVector))) true true "(R=0.000000,G=0.660000,B=1.000000,A=1.000000)" 2.0 "Dot"))

(fn CrossProduct
  (bind _returnvalue (Transformation|GetActorLocation))
  (Rendering|Debug|DrawDebugLine _returnvalue (+ _returnvalue (* (Math|Vector|CrossProduct (Transformation|GetActorForwardVector (Variables|Default|GetPlayer)) (Transformation|GetActorForwardVector)) 2e+02)) "(R=1.000000,G=0.000000,B=0.377531,A=1.000000)" 0.0 15.0))