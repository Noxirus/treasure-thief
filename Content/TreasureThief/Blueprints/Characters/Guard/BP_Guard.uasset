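; BP_Guard is a guard NPC that prints a joke line of dialogue when interacted with.
; On BeginPlay it caches the player goblin and its AIC_Guard controller.
; It exposes patrol helpers that return the current spline point on its route, wrapping by modulo, and advance the index.
; Dot and cross product functions visualize facing debug info but are not called here, and a delayed SetTarget call is unwired.
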(event EventBeginInteraction
  (params (Instigator :type BP%20Player%20Goblin%20Object%20Reference))
  (CallFunction|TalktoGuard))

(event EventBeginPlay
  (Utilities|FlowControl|Sequence
    (:then_0
      (bind _returnvalue (Actor|GetActorOfClass "/Game/TreasureThief/Blueprints/Characters/PlayerGoblin/BP_PlayerGoblin.BP_PlayerGoblin_C"))
      (Variables|Default|SetPlayer _returnvalue))
    (:then_1
      (bind _asaic_guard (Utilities|Casting|CastToAIC_Guard (Pawn|GetController)))
      (bind _output_get (Variables|Default|SetAIController _asaic_guard)))))

(fn ConstructionScript)

(fn DotProduct
  (Development|PrintString (Utilities|String|ToString(Float) (Math|Vector|DotProduct (Math|Vector|Normalize (- (Transformation|GetActorLocation (Variables|Default|GetPlayer)) (Transformation|GetActorLocation))) (Transformation|GetActorForwardVector))) true true "(R=0.000000,G=0.660000,B=1.000000,A=1.000000)" 2.0 "Dot"))

(fn CrossProduct
  (bind _returnvalue (Transformation|GetActorLocation))
  (Rendering|Debug|DrawDebugLine _returnvalue (+ _returnvalue (* (Math|Vector|CrossProduct (Transformation|GetActorForwardVector (Variables|Default|GetPlayer)) (Transformation|GetActorForwardVector)) 2e+02)) "(R=1.000000,G=0.000000,B=0.377531,A=1.000000)" 0.0 15.0))

(fn TalktoGuard
  (Development|PrintString "I used to be an adventurer like you, then I took an arrow to the elbow"))

(fn CurrentSplineDestination
  (bind _patrolroute (Variables|Default|GetPatrolRoute))
  (bind _splinepath (Variables|/Game/TreasureThief/Blueprints/Characters/Guard/AI/BP_PatrolRoute.BP_PatrolRoute_C|GetSplinePath _patrolroute))
  (return (Spline|GetLocationatSplinePoint _splinepath (Math|Integer|%(Integer) (Variables|Default|GetPatrolIndex) (Spline|GetNumberOfSplinePoints _splinepath)) "World")))

(fn IncrementPatrol
  (Math|Integer|IncrementInt (Variables|Default|GetPatrolIndex)))