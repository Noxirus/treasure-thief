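; Player-controlled goblin character for TreasureThief, with Enhanced Input movement, camera look, jumping and melee attacks.
; A state check gates movement and attacks, which play a randomly chosen montage section.
; Weapon overlaps spawn and trigger an FS_MasterField actor; collision starts disabled and nothing here re-enables it or resets the attack state.
; Interact is only a debug box trace, offset from world origin rather than the actor's location.
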(event Input|EnhancedActionEvents|EnhancedInputActionIA_Interact
  (params (ActionValue :type Boolean) (ElapsedSeconds :type Float%20%28double-precision%29) (TriggeredSeconds :type Float%20%28double-precision%29) (InputAction :type Input%20Action%20Object%20Reference :default "/Game/TreasureThief/Input/IA_Interact.IA_Interact"))
  (bind _returnvalue (Transformation|GetActorForwardVector))
  (bind _returnvalue_2 (* _returnvalue 1.5e+02))
  (bind _returnvalue_3 (+ "" _returnvalue_2))
  (:Started
    (Development|PrintString "Interaction Pressed")
    (Class|KismetSystemLibrary|BoxTraceSingleforObjects _returnvalue_3 _returnvalue_3 "40.000000,40.000000,40.000000" "0, 0, 0" (Utilities|Array|MakeArray "ObjectTypeQuery3") false 0 "ForDuration" true)))

(event EventBeginPlay
  (CallFunction|SetupInput)
  (CallFunction|SetWeaponCollision "NoCollision"))

(event Input|EnhancedActionEvents|EnhancedInputActionIA_Jump
  (params (ActionValue :type Boolean) (ElapsedSeconds :type Float%20%28double-precision%29) (TriggeredSeconds :type Float%20%28double-precision%29) (InputAction :type Input%20Action%20Object%20Reference :default "/Game/TreasureThief/Input/IA_Jump.IA_Jump"))
  (:Started
    (Character|Jump)))

(event Input|EnhancedActionEvents|EnhancedInputActionIA_Move
  (params (ActionValue :type Vector%202D%20Structure) (ElapsedSeconds :type Float%20%28double-precision%29) (TriggeredSeconds :type Float%20%28double-precision%29) (InputAction :type Input%20Action%20Object%20Reference :default "/Game/TreasureThief/Input/IA_Move.IA_Move"))
  (if (CallFunction|CanAct)
    (CallFunction|MoveCharacter ActionValue)))

(event Input|EnhancedActionEvents|EnhancedInputActionIA_Look
  (params (ActionValue :type Vector%202D%20Structure) (ElapsedSeconds :type Float%20%28double-precision%29) (TriggeredSeconds :type Float%20%28double-precision%29) (InputAction :type Input%20Action%20Object%20Reference :default "/Game/TreasureThief/Input/IA_Look.IA_Look"))
  (Pawn|Input|AddControllerYawInput (.x ActionValue))
  (Pawn|Input|AddControllerPitchInput (.y ActionValue)))

(event OnComponentBeginOverlap(WeaponCollision)
  (params (OverlappedComponent :type Primitive%20Component%20Object%20Reference) (OtherActor :type Actor%20Object%20Reference) (OtherComp :type Primitive%20Component%20Object%20Reference) (OtherBodyIndex :type Integer) (bFromSweep :type Boolean) (SweepResult :type Hit%20Result%20Structure%20%28by%20ref%29))
  (Development|PrintString (Utilities|GetDisplayName OtherActor))
  (bind _returnvalue (Game|SpawnActorfromClass "/Engine/EditorResources/FieldNodes/FS_MasterField.FS_MasterField_C" (Transformation|GetWorldTransform (Variables|Default|GetWeaponCollision)) "Undefined" "MultiplyWithRoot" 0 0))
  (Default|CETrigger _returnvalue))

(event Input|EnhancedActionEvents|EnhancedInputActionIA_Attack
  (params (ActionValue :type Boolean) (ElapsedSeconds :type Float%20%28double-precision%29) (TriggeredSeconds :type Float%20%28double-precision%29) (InputAction :type Input%20Action%20Object%20Reference :default "/Game/TreasureThief/Input/IA_Attack.IA_Attack"))
  (:Started
    (if (CallFunction|CanAct)
      (Variables|Default|SetCurrentState "NewEnumerator1")
      (Animation|Montage|PlayMontage (Variables|Character|GetMesh) "/Game/TreasureThief/Assets/Characters/Goblin/Animations/AM_GoblinAttack.AM_GoblinAttack" 1.0 0.0 (.OutItem (Utilities|Array|Random (Variables|Default|GetAttackStrings)))))))

(fn ConstructionScript
  (Transformation|AttachComponentToComponent (Variables|Default|GetWeaponMesh) (Variables|Character|GetMesh) "LeftHandSocket" "KeepRelative" "KeepRelative" "KeepRelative" true))

(fn MoveCharacter
  (params (MoveAxis :type Vector%202D%20Structure))
  (bind _returnvalue (Pawn|GetControlRotation :!class /Script/Engine.Pawn))
  (Pawn|Input|AddMovementInput (Math|Vector|GetRightVector (Math|Rotator|MakeRotator (.roll _returnvalue) 0.0 (.yaw _returnvalue))) (.x MoveAxis) false)
  (Pawn|Input|AddMovementInput (Math|Vector|GetForwardVector (Math|Rotator|MakeRotator 0.0 0.0 (.yaw (Pawn|GetControlRotation :!class /Script/Engine.Pawn)))) (.y MoveAxis) false))

(fn SetupInput
  (bind _asplayer_controller (Utilities|Casting|CastToPlayerController (Pawn|GetController)))
  (Input|AddMappingContext (PlayerController|LocalPlayerSubsystems|GetEnhancedInputLocalPlayerSubsystem _asplayer_controller) "/Game/TreasureThief/Input/IMC_Default.IMC_Default" 0 "(bIgnoreAllPressedKeysUntilRelease=True,bForceImmediately=False,bNotifyUserSettings=False)"))

(fn SetWeaponCollision
  (params (CollisionState :type ECollisionEnabled%20Enum :default "NoCollision"))
  (Collision|SetCollisionEnabled (Variables|Default|GetWeaponCollision) CollisionState))

(fn CanAct
  (return (Utilities|Enum|Equal(Enum) (Variables|Default|GetCurrentState) "NewEnumerator0")))

(fn SetCharacterState
  (params (CurrentState :type E_CharacterStates%20Enum :default "NewEnumerator0"))
  (Variables|Default|SetCurrentState CurrentState))

(fn MultiLineTrace
  (bind _outhits (Collision|MultiLineTraceByChannel (Transformation|GetActorLocation) (+ (Transformation|GetActorLocation) (* (Transformation|GetActorForwardVector) 1e+03)) "TraceTypeQuery2" false 0 "ForDuration"))
  (for _array_element _outhits
    (Development|PrintString (Utilities|GetDisplayName (.HitActor (Collision|BreakHitResult _array_element))))))